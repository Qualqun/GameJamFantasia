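; BP_Key is a key actor, a child Blueprint under Carryable, that reports its pickup state to the player character.
; On BeginPlay it runs the parent logic, caches the player pawn as BP_C_PlayerCharacter and binds to its own PickUpDIspatch dispatcher.
; When that dispatcher fires, it relays the HasKey value through the player character's KeyEvent.
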(event Custom|PickUpDIspatch_Event
  (params (HasKey :type Boolean))
  (Default|CallKeyEvent (Variables|Default|GetPlayerCharacter) HasKey))

(event EventBeginPlay
  (|CallParentFunction)
  (Utilities|FlowControl|Sequence
    (:then_0
      (bind _asbp_c_player_character (Utilities|Casting|CastToBP_C_PlayerCharacter (Game|Player|GetPlayerPawn 0)))
      (Variables|Default|SetPlayerCharacter _asbp_c_player_character))
    (:then_1
      (EventDispatchers|AssignPickUpDIspatch (delegate Custom|PickUpDIspatch_Event)))))

(event Collision|EventActorBeginOverlap
  (params (OtherActor :type Actor%20Object%20Reference)))

(event EventTick
  (params (DeltaSeconds :type Float%20%28single-precision%29))
  (|CallParentFunction DeltaSeconds) ; This node is disabled and will not be called.\nDrag off pins to build functionality.
)

(fn ConstructionScript
  (|CallParentFunction))