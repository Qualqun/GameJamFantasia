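; BP_Pushable is a child actor Blueprint for a prop the player can push across a 100-unit tile grid.
; PushObject requires a finished lerp and a nearby player, then flags a push if the neighboring tile in that direction has type 3.
; GetTileType indexes AGrid by snapped position.
; GetTileSeason, uncalled here, traces down for a BP_ATile with debug output; the movement itself is absent from these graphs.
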(event EventBeginPlay
  (|CallParentFunction) ; This node is disabled and will not be called.\nDrag off pins to build functionality.
)

(event Collision|EventActorBeginOverlap
  (params (OtherActor :type Actor%20Object%20Reference)))

(event EventTick
  (params (DeltaSeconds :type Float%20%28single-precision%29)))

(event EventPushObject
  (if (Variables|Default|GetLerpIsEnd)
    (bind (_isclose _direction) (CallFunction|ClosedtoPlayer))
    (if _isclose
      (bind _output_get (Variables|Default|SetDirection _direction))
      (bind _tile (CallFunction|GetTileType (+ (* _output_get 100) (+ (Transformation|GetActorLocation) (Variables|Default|GetOffSet)))))
      (if (== _tile 3)
        (Variables|Default|SetIsPushed true)
        (Variables|Default|SetLerpIsEnd false)))))

(fn ConstructionScript
  (|CallParentFunction))

(fn GetTileType
  (params (Pos :type Vector))
  (bind _returnvalue (Class|KismetMathLibrary|VectorSnappedtoGrid Pos 1e+02))
  (bind _returnvalue_2 (/ _returnvalue 100))
  (return (.tiletype (Utilities|Array|Get(acopy) (.row (Utilities|Array|Get(acopy) (Variables|/Game/Core/Blueprints/Actor/Parent/BP_AGrid.BP_AGrid_C|GetTiles (Variables|Default|GetAGrid)) (Math|Float|Truncate (.x _returnvalue_2)))) (Math|Float|Truncate (.y _returnvalue_2))))))

(fn GetTileSeason
  (params (Pos :type Vector))
  (bind _outhit (Collision|LineTraceByChannel Pos (+ Pos (* (Math|Vector|VectorDown) 200)) "TraceTypeQuery1" false (Utilities|Array|MakeArray (Variables|Default|GetPlayerPawn)) "ForDuration"))
  (bind _asbp_atile (Utilities|Casting|CastToBP_ATile (.hitactor _outhit))
    (:then
      (Development|PrintString (Utilities|String|EnumtoString (Variables|/Game/Core/Blueprints/Actor/Parent/BP_ATile.BP_ATile_C|GetSeason _asbp_atile)))
      (return _asbp_atile true))
    (:CastFailed
      (Development|PrintString "ATile cast failed")
      (return 0 false))))