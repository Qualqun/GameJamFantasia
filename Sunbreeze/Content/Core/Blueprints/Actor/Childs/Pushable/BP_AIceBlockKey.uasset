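; Pushable ice block that melts on a tile of a specific season and leaves a key behind.
; A looping timer from BeginPlay checks the season of the tile beneath it, but only once the inherited lerp has ended.
; On a match, it stops the timer and plays a timeline that scales the ice mesh's height, then spawns BP_Key in place and destroys itself.
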(event Custom|CheckSeason
  (if (Variables|Default|GetLerpIsEnd)
    (bind _tile (CallFunction|GetTileSeason (Transformation|GetActorLocation)))
    (if (== (Variables|/Game/Core/Blueprints/Actor/Parent/BP_ATile.BP_ATile_C|GetSeason _tile) 3)
      (Utilities|Time|ClearandInvalidateTimerbyHandle (stale EventBeginPlay _returnvalue))
      (bind _melt (Timeline|Melting Play)
        (:Update
          (Transformation|SetRelativeScale3D (Variables|Default|GetIceBloc) (Math|Vector|MakeVector 1.0 1.0 _melt)))
        (:Finished
          (Game|SpawnActorfromClass "/Game/Core/Blueprints/Actor/Childs/Carryable/BP_Key.BP_Key_C" (Math|Transform|MakeTransform (Transformation|GetActorLocation) "0, 0, 0" "1.000000,1.000000,1.000000") "Undefined" "MultiplyWithRoot" 0 0)
          (Actor|DestroyActor))))))

(event EventBeginPlay
  (|CallParentFunction)
  (bind _returnvalue (Utilities|Time|SetTimerbyEvent (delegate Custom|CheckSeason) 0.25 true)))

(fn ConstructionScript
  (|CallParentFunction))