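; Pushable rock actor whose hole behaviour moves it into a hole, changes the tile below, then destroys itself.
; Two chained timelines lerp it one tile along the push direction, call SetTileMovable, then lower it by one tile distance.
; A short downward debug-drawn line trace then finds the BP_ATile beneath, switches its type and refreshes it through ChangeOnType.
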(event EventHoleBehaviour
  (Variables|Default|SetLerpIsEnd false)
  (bind _output_get (Variables|Default|SetActualPos (Transformation|GetActorLocation)))
  (bind _lerp (Timeline|UpHole PlayFromStart)
    (:Update
      (Transformation|SetActorLocation (Math|Vector|Lerp(Vector) _output_get (+ _output_get (* (Variables|Default|GetDirection) (Variables|Default|GetDistNextTile))) _lerp) false false))
    (:Finished
      (CallFunction|SetTileMovable)
      (bind _output_get_2 (Variables|Default|SetActualPos (+ _output_get (* (Variables|Default|GetDirection) (Variables|Default|GetDistNextTile)))))
      (bind _lerp_2 (Timeline|DownHole PlayFromStart)
        (:Update
          (Transformation|SetActorLocation (Math|Vector|Lerp(Vector) _output_get_2 (+ _output_get_2 (* (Math|Vector|VectorDown) (Variables|Default|GetDistNextTile))) _lerp_2) false false))
        (:Finished
          (bind _outhit (Collision|LineTraceByChannel (Math|Vector|Lerp(Vector) _output_get_2 (+ _output_get_2 (* (Math|Vector|VectorDown) (Variables|Default|GetDistNextTile))) _lerp_2) (+ (Math|Vector|Lerp(Vector) _output_get_2 (+ _output_get_2 (* (Math|Vector|VectorDown) (Variables|Default|GetDistNextTile))) _lerp_2) (Math|Vector|VectorDown)) "TraceTypeQuery1" false 0 "ForDuration" true "(R=1.000000,G=0.856351,B=0.000000,A=1.000000)" "(R=0.169972,G=0.141087,B=1.000000,A=1.000000)"))
          (bind _asbp_atile (Utilities|Casting|CastToBP_ATile (.hitactor _outhit)))
          (Variables|/Game/Core/Blueprints/Actor/Parent/BP_ATile.BP_ATile_C|SetTileType _asbp_atile "NewEnumerator3")
          (Default|ChangeonType _asbp_atile)
          (Actor|DestroyActor))))))

(fn ConstructionScript
  (|CallParentFunction))