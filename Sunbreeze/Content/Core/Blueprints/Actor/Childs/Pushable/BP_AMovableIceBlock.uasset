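; Movable ice block that the player pushes across the tile grid by standing in an orthogonally adjacent cell.
; Each Tick compares grid positions and starts a push away from the player if BP_AGrid reports the required tile type ahead.
; A timeline lerps the block one step, then a downward trace reads the next BP_ATile's season to decide whether it keeps sliding, without rechecking tile type.
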(event EventTick
  (params (DeltaSeconds :type Float%20%28single-precision%29))
  (CallFunction|PushObject)
  (if (Variables|Default|GetIsPushed)
    (Variables|Default|SetIsPushed false)
    (bind _output_get (Variables|Default|SetActualPos (Transformation|GetActorLocation)))
    (bind _lerp (Timeline|LerpToPos PlayFromStart)
      (:Update
        (Transformation|SetActorLocation (Math|Vector|Lerp(Vector) _output_get (+ _output_get (* (Variables|Default|GetDirection) (Variables|Default|GetDistNextCase))) _lerp) false true))
      (:Finished
        ;[0.15 0.15 0.15 0.5] Insert ice logic
        (Variables|Default|SetLerpIsEnd true)
        (bind (_tile _isvalin) (CallFunction|GetTileSeason (+ (Transformation|GetActorLocation) (* (Variables|Default|GetDirection) 100))))
        (Variables|Default|SetIsPushed (== (== (Variables|/Game/Core/Blueprints/Actor/Parent/BP_ATile.BP_ATile_C|GetSeason _tile) 0) _isvalin))))))

(event EventBeginPlay
  (Variables|Default|SetPlayerPawn (Game|Player|GetPlayerPawn 0))
  (bind _outactors (Actor|GetAllActorsOfClass "/Game/Core/Blueprints/Actor/Parent/BP_AGrid.BP_AGrid_C"))
  (Variables|Default|SetAGrid (Utilities|Array|Get(acopy) _outactors))
  (CallFunction|SetGridPos))

(fn ConstructionScript
  (|CallParentFunction))

(fn GetTileSeason
  (params (Pos :type Vector))
  (bind _outhit (Collision|LineTraceByChannel Pos (+ Pos (* (Math|Vector|VectorDown) 200)) "TraceTypeQuery1" false 0 "None"))
  (bind _asbp_atile (Utilities|Casting|CastToBP_ATile (.hitactor _outhit))
    (:then
      (Development|PrintString (Utilities|String|EnumtoString (Variables|/Game/Core/Blueprints/Actor/Parent/BP_ATile.BP_ATile_C|GetSeason _asbp_atile)))
      (return _asbp_atile true))
    (:CastFailed
      (Development|PrintString "ATile cast failed")
      (return 0 false))))

(fn GetTileType
  (params (Pos :type Vector))
  (bind _agrid (Variables|Default|GetAGrid))
  (bind _gridposition (Default|WorldtoGrid _agrid Pos))
  (return (.tiletype (Utilities|Array|Get(acopy) (.row (Utilities|Array|Get(acopy) (Variables|/Game/Core/Blueprints/Actor/Parent/BP_AGrid.BP_AGrid_C|GetTiles (Variables|Default|GetAGrid)) (Math|Float|Truncate (.x _gridposition)))) (Math|Float|Truncate (.y _gridposition))))))

(fn PushObject
  (bind _pos (Utilities|GetGridPlayerPos))
  (bind _position (Utilities|GetPropGridPos))
  (bind _returnvalue (- _pos _position))
  (if (== (Math|Vector|VectorLength _returnvalue) 1.0)
    (if (Variables|Default|GetLerpIsEnd)
      (bind _output_get (Variables|Default|SetDirection (* _returnvalue -1)))
      (bind _tile (CallFunction|GetTileType (+ (* _output_get 100) (Transformation|GetActorLocation))))
      (if (== 3 _tile)
        (Variables|Default|SetIsPushed true)
        (Variables|Default|SetLerpIsEnd false)
        (return)))))