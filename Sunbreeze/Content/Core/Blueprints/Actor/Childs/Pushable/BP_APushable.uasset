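; Pushable object that the player shoves one tile at a time across a tile grid.
; PushObject takes its direction from the player check, box-checks the next tile for other pushables, plays a sound and lerps over via a timeline.
; Downward traces read tile type and season: the ice season keeps it sliding while the path allows, and holes call the empty HoleBehaviour hook.
; Traces and overlap checks draw debug shapes.
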(event Custom|HoleBehaviour)

(event EventBeginPlay
  (|CallParentFunction)
  (bind _outactors (Actor|GetAllActorsOfClass "/Game/Core/Blueprints/Actor/Parent/BP_AGrid.BP_AGrid_C"))
  (Variables|Default|SetAGrid (Utilities|Array|Get(acopy) _outactors)))

(event EventPushObject
  (bind _returnvalue (Transformation|GetActorLocation))
  (bind _returnvalue_2 (Transformation|GetActorLocation))
  (if (Variables|Default|GetLerpIsEnd)
    (bind (_isclose _direction) (CallFunction|ClosedtoPlayer))
    (if _isclose
      (bind _output_get (Variables|Default|SetDirection _direction))
      (bind _hadobstacle (CallFunction|NexTileAvailable (+ (* _output_get 100) _returnvalue)))
      (if (not _hadobstacle)
        (Class|FMODBlueprintStatics|PlayEventAttached "/Game/FMOD/Events/PushBlocks.PushBlocks" (Variables|Default|GetRoot) "None" _returnvalue "KeepWorldPosition")
        (bind _tile (CallFunction|GetTileType (+ (* _output_get 100) _returnvalue) :!label _label))
        (if (Utilities|Enum|Equal(Enum) _tile "NewEnumerator3")
          (Variables|Default|SetLerpIsEnd false)
          (bind _output_get_2 (Variables|Default|SetActualPos (Transformation|GetActorLocation)))
          (bind _lerp (Timeline|Timeline PlayFromStart)
            (:Update
              (Transformation|SetActorLocation (Math|Vector|Lerp(Vector) _output_get_2 (+ _output_get_2 (* (Variables|Default|GetDirection) (Variables|Default|GetDistNextTile))) _lerp) false false))
            (:Finished
              (bind _tile_2 (CallFunction|GetTileSeason _returnvalue_2))
              (if (== (Variables|/Game/Core/Blueprints/Actor/Parent/BP_ATile.BP_ATile_C|GetSeason _tile_2) 0)
                ;[0.15 0.15 0.15 0.5] Insert ice logic
                (bind (_tile_3 _isvalid _isrock) (CallFunction|GetTileSeason (+ _returnvalue_2 (* (Variables|Default|GetDirection) (Variables|Default|GetDistNextTile)))))
                (bind _hadobstacle_2 (CallFunction|NexTileAvailable (+ _returnvalue_2 (* (Variables|Default|GetDirection) (Variables|Default|GetDistNextTile)))))
                (if _hadobstacle_2
                  (Variables|Default|SetLerpIsEnd true)
                  (else
                    (bind _tile_4 (CallFunction|GetTileType (+ _returnvalue_2 (* (Variables|Default|GetDirection) (Variables|Default|GetDistNextTile)))))
                    (Variables|Default|SetLerpIsEnd true)
                    (if (== true (== 3 _tile_4))
                      (goto _label)
                      (elif (== _tile_4 1)
                        (CallFunction|HoleBehaviour)))))
                (else
                  (Variables|Default|SetLerpIsEnd true)))))
          (elif (Utilities|Enum|Equal(Enum) _tile "NewEnumerator1")
            (CallFunction|HoleBehaviour)))))))

(fn ConstructionScript
  (|CallParentFunction))

(fn GetTileType
  (params (Pos :type Vector))
  (bind _outhit (Collision|LineTraceByChannel Pos (+ Pos (* (Math|Vector|VectorDown) 500)) "TraceTypeQuery1" false (Utilities|Array|MakeArray (Variables|Default|GetPlayerPawn)) "ForDuration" true "(R=0.939790,G=0.947735,B=1.000000,A=1.000000)" "(R=0.043898,G=0.000000,B=1.000000,A=1.000000)" 5e+01))
  (bind _asbp_atile (Utilities|Casting|CastToBP_ATile (.hitactor _outhit)))
  (return (Variables|/Game/Core/Blueprints/Actor/Parent/BP_ATile.BP_ATile_C|GetTileType _asbp_atile)))

(fn GetTileSeason
  (params (Pos :type Vector))
  (bind _outhit (Collision|LineTraceByChannel Pos (+ Pos (* (Math|Vector|VectorDown) 200)) "TraceTypeQuery1" false (Utilities|Array|MakeArray (Variables|Default|GetPlayerPawn)) "ForDuration"))
  (bind _asbp_atile (Utilities|Casting|CastToBP_ATile (.hitactor _outhit)))
  (return _asbp_atile true false))

(fn SetTileMovable
  (bind _actualpos (Variables|Default|GetActualPos))
  (bind _grid (Variables|Default|GetGrid))
  (bind _returnvalue (Class|KismetMathLibrary|VectorSnappedtoGrid _actualpos 1e+02))
  (bind _tiles (Variables|/Game/Core/Blueprints/Actor/Parent/BP_AGrid.BP_AGrid_C|GetTiles _grid))
  (bind _returnvalue_2 (/ _returnvalue 100))
  (bind _returnvalue_3 (Math|Float|Truncate (.y _returnvalue_2)))
  (bind _returnvalue_4 (Math|Float|Truncate (.x _returnvalue_2)))
  (bind _output (Utilities|Array|Get(acopy) _tiles _returnvalue_4))
  (bind _output_2 (Utilities|Array|Get(acopy) (.row _output) _returnvalue_3))
  (bind _structout (Utilities|Struct|SetmembersinTileData _output_2 "NewEnumerator3"))
  (|SetBy-RefVar _output_2 _structout)
  (return))

(fn NexTileAvailable
  (params (Pos :type Vector))
  (bind _returnvalue (Math|Vector|VectorUp))
  (bind _boxextend (Variables|Default|GetBoxExtend))
  (bind _returnvalue_2 (* _returnvalue 50))
  (bind _returnvalue_3 (+ Pos _returnvalue_2))
  (Rendering|Debug|DrawDebugBox _returnvalue_3 _boxextend "(R=0.000000,G=0.102267,B=1.000000,A=1.000000)" "0, 0, 0" 5.0 0.0)
  (bind _outactors (Collision|BoxOverlapActors _returnvalue_3 _boxextend (Utilities|Array|MakeArray "ObjectTypeQuery1" "ObjectTypeQuery2" "ObjectTypeQuery4") "BP_APushable_C" (Utilities|Array|MakeArray self) :!class /Script/Engine.KismetSystemLibrary))
  (return (> (Utilities|Array|Length _outactors) 0)))