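; Pushable actor that inverts the season of the tiles around it between winter and summer.
; A looping timer restores the tiles changed on the previous pass, then sphere-overlaps tiles within Range, flips their season and refreshes them.
; HoleBehaviour chains two timelines to slide it one tile along Direction and drop it down, then retypes the traced tile below, plays the fall event and destroys the actor.
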(event Custom|ChangeSeasonTiles
  (bind _tileschangedonlast (Variables|Default|GetTilesChangedOnLast))
  (for _array_element _tileschangedonlast
    (Variables|/Game/Core/Blueprints/Actor/Parent/BP_ATile.BP_ATile_C|SetSeason _array_element (Variables|/Game/Core/Blueprints/Actor/Parent/BP_ATile.BP_ATile_C|GetoriginalSeason _array_element))
    (Default|ChangeonType _array_element))
  (Utilities|Array|Clear _tileschangedonlast)
  (bind _outactors (Collision|SphereOverlapActors (Transformation|GetActorLocation) (Variables|Default|GetRange) (Utilities|Array|MakeArray "ObjectTypeQuery1") "/Game/Core/Blueprints/Actor/Parent/BP_ATile.BP_ATile_C"))
  (for _array_element_2 _outactors
    (bind _asbp_atile (Utilities|Casting|CastToBP_ATile _array_element_2))
    (Utilities|Array|Add (Variables|Default|GetTilesChangedOnLast) _asbp_atile)
    (Variables|/Game/Core/Blueprints/Actor/Parent/BP_ATile.BP_ATile_C|SetSeason _asbp_atile (Utilities|Select :Index (Variables|/Game/Core/Blueprints/Actor/Parent/BP_ATile.BP_ATile_C|GetSeason _asbp_atile) :NewEnumerator0 "NewEnumerator3" :NewEnumerator1 "NewEnumerator3" :NewEnumerator2 "NewEnumerator0" :NewEnumerator3 "NewEnumerator0"))
    (Default|ChangeonType _asbp_atile)))

(event EventBeginPlay
  (|CallParentFunction)
  (Utilities|Time|SetTimerbyEvent (delegate Custom|ChangeSeasonTiles) (Variables|Default|GetTimeCheck) true true))

(event EventHoleBehaviour
  (bind _output_get (Variables|Default|SetActualPos (Transformation|GetActorLocation)))
  (bind _lerp (Timeline|Timeline_0 PlayFromStart)
    (:Update
      (Transformation|SetActorLocation (Math|Vector|Lerp(Vector) _output_get (+ _output_get (* (Variables|Default|GetDirection) (Variables|Default|GetDistNextTile))) _lerp) false false))
    (:Finished
      (CallFunction|SetTileMovable)
      (bind _output_get_2 (Variables|Default|SetActualPos (+ _output_get (* (Variables|Default|GetDirection) (Variables|Default|GetDistNextTile)))))
      (bind _lerp_2 (Timeline|Timeline_1 PlayFromStart)
        (:Update
          (Transformation|SetActorLocation (Math|Vector|Lerp(Vector) _output_get_2 (+ _output_get_2 (* (Math|Vector|VectorDown) (Variables|Default|GetDistNextTile))) _lerp_2) false false))
        (:Finished
          (bind _outhit (Collision|LineTraceByChannel (Math|Vector|Lerp(Vector) _output_get_2 (+ _output_get_2 (* (Math|Vector|VectorDown) (Variables|Default|GetDistNextTile))) _lerp_2) (+ (Math|Vector|Lerp(Vector) _output_get_2 (+ _output_get_2 (* (Math|Vector|VectorDown) (Variables|Default|GetDistNextTile))) _lerp_2) (Math|Vector|VectorDown)) "TraceTypeQuery1" false 0 "ForDuration" true "(R=1.000000,G=0.856351,B=0.000000,A=1.000000)" "(R=0.169972,G=0.141087,B=1.000000,A=1.000000)"))
          (bind _asbp_atile (Utilities|Casting|CastToBP_ATile (.hitactor _outhit)))
          (Variables|/Game/Core/Blueprints/Actor/Parent/BP_ATile.BP_ATile_C|SetTileType _asbp_atile "NewEnumerator3")
          (Default|ChangeonType _asbp_atile)
          (Class|FMODBlueprintStatics|PlayEventAttached "/Game/FMOD/Events/BlockFalls.BlockFalls" (Variables|Default|GetRoot) "None" (Transformation|GetActorLocation) "KeepWorldPosition")
          (Actor|DestroyActor))))))

(fn ConstructionScript
  (|CallParentFunction))