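; BP_Seasonal is an actor that flips the season of the tiles around it, turning winter tiles to summer and summer tiles to winter.
; A looping timer restores the previously changed tiles to their original season, then sphere-traces at the actor's location within RadiusSeasonal.
; Each BP_ATile hit is recorded for the next reset, flipped and refreshed through ChangeOnType, so the effect follows the actor.
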(event EventBeginPlay
  (|CallParentFunction)
  (Utilities|Time|SetTimerbyFunctionName 0 "ChangeAroundState" (Variables|Default|GetTimeToTrace) true true))

(event Collision|EventActorBeginOverlap
  (params (OtherActor :type Actor%20Object%20Reference))
  (|CallParentFunction OtherActor) ; This node is disabled and will not be called.\nDrag off pins to build functionality.
)

(event EventTick
  (params (DeltaSeconds :type Float%20%28single-precision%29))
  (|CallParentFunction DeltaSeconds))

(fn ConstructionScript
  (|CallParentFunction))

(fn ChangeAroundState
  ;[0.15 0.15 0.15 0.5] Set back to last season
  (for _array_element (Variables|Default|GetTilesChangedLast)
    (Variables|/Game/Core/Blueprints/Actor/Parent/BP_ATile.BP_ATile_C|SetSeason _array_element (Variables|/Game/Core/Blueprints/Actor/Parent/BP_ATile.BP_ATile_C|GetoriginalSeason _array_element))
    (Default|ChangeonType _array_element))
  ;[0.15 0.15 0.15 0.5] reset vector
  (Utilities|Array|Clear (Variables|Default|GetTilesChangedLast))
  (bind _outhits (CallFunction|SphereTraceatActorLocation))
  (for _array_element_2 _outhits
    (if (== (Utilities|GetClass (.HitActor (Collision|BreakHitResult _array_element_2))) "/Game/Core/Blueprints/Actor/Parent/BP_ATile.BP_ATile_C")
      (bind _asbp_atile (Utilities|Casting|CastToBP_ATile (.HitActor (Collision|BreakHitResult _array_element_2))))
      (Utilities|Array|Add (Variables|Default|GetTilesChangedLast) _asbp_atile)
      (CallFunction|ApplyTransformationonTile _asbp_atile))))

(fn ApplyTransformationonTile
  (params (tile :type BP%20A%20Tile%20Object%20Reference))
  (Variables|/Game/Core/Blueprints/Actor/Parent/BP_ATile.BP_ATile_C|SetSeason tile (Utilities|Select :Index (Variables|/Game/Core/Blueprints/Actor/Parent/BP_ATile.BP_ATile_C|GetSeason tile) :NewEnumerator0 "NewEnumerator3" :NewEnumerator1 "NewEnumerator3" :NewEnumerator2 "NewEnumerator0" :NewEnumerator3 "NewEnumerator0"))
  (Default|ChangeonType tile))

(fn SphereTraceatActorLocation
  (bind _returnvalue (Transformation|GetActorLocation))
  (bind _outhits (Collision|MultiSphereTraceForObjects _returnvalue _returnvalue (Variables|Default|GetRadiusSeasonal) (Utilities|Array|MakeArray "ObjectTypeQuery1" "ObjectTypeQuery2") true 0 "None" true "(R=1.000000,G=0.000000,B=0.000000,A=1.000000)" "(R=0.000000,G=1.000000,B=0.000000,A=1.000000)" 1.0))
  (return _outhits))