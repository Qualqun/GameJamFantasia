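; Parent Blueprint for carryable actors that are lifted onto the player, apparently to sit above the head.
; PickUp stores the start location, then a timeline lerps the actor to the player pawn's location plus a PlayerHeight Z offset and sets Picked.
; While Picked, Tick adds PlayerHeight to the actor's own location each frame rather than following the pawn.
; The PlayerHeight bounds calculation and timer calls are unconnected.
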(event EventBeginPlay
  (|CallParentFunction))

(event EventTick
  (params (DeltaSeconds :type Float%20%28single-precision%29))
  ;[0.15 0.15 0.15 0.5] Snap headPlayer
  (if (Variables|Default|GetPicked)
    (Transformation|SetActorLocation (+ (Transformation|GetActorLocation) (Math|Vector|MakeVector 0.0 0.0 (Variables|Default|GetPlayerHeight))) false false)))

(event EventPickUp
  (Variables|Default|SetStartActorPos (Transformation|GetActorLocation))
  (bind _time (Timeline|LerpPickUp PlayFromStart)
    (:Update
      (Transformation|SetActorLocation (Math|Vector|Lerp(Vector) (Variables|Default|GetStartActorPos) (+ (Transformation|GetActorLocation (Variables|Default|GetPlayerPawn)) (Math|Vector|MakeVector 0.0 0.0 (Variables|Default|GetPlayerHeight))) _time) false false))
    (:Finished
      (Variables|Default|SetPicked true))))

(fn ConstructionScript
  (|CallParentFunction))