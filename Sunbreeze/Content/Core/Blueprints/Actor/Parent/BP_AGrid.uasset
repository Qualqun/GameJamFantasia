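; BP_AGrid is a parent grid actor that builds a 16x10 tile map on BeginPlay from its Tiles array of rows.
; The construction script pre-fills an empty Tiles array with 16 entries.
; GenerateGrid spawns BP_ATile actors 100 units apart from world origin, sets each tile's type and a season split between the two X halves, then calls Init.
; Helper functions convert between world and grid coordinates.
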(event EventBeginPlay
  (CallFunction|GenerateGrid))

(fn ConstructionScript
  (CallFunction|EmptyInit))

(fn GenerateGrid
  (Utilities|Array|Resize (Variables|Default|GetTiles) 16)
  (for _index (range 0 15)
    (for _index_2 (range 0 9)
      (bind _returnvalue (Game|SpawnActorfromClass "/Game/Core/Blueprints/Actor/Parent/BP_ATile.BP_ATile_C" (Math|Transform|MakeTransform (Math|Vector|MakeVector (Math|Conversions|ToFloat(Integer) (* _index 100)) (Math|Conversions|ToFloat(Integer) (* _index_2 100)) 0.0) "0, 0, 0" "1.000000,1.000000,1.000000") "Undefined" "MultiplyWithRoot" 0 0))
      (Variables|/Game/Core/Blueprints/Actor/Parent/BP_ATile.BP_ATile_C|SetTileType _returnvalue (.tiletype (Utilities|Array|Get(acopy) (.row (Utilities|Array|Get(acopy) (Variables|Default|GetTiles) _index)) _index_2)))
      (Variables|/Game/Core/Blueprints/Actor/Parent/BP_ATile.BP_ATile_C|SetSeason _returnvalue (select (<= _index 7) "NewEnumerator0" "NewEnumerator3"))
      (Default|Init _returnvalue))))

(fn WorldtoGrid
  (params (WorldPosition :type Vector))
  (return (/ WorldPosition "100.000000,100.000000,100.000000")))

(fn EmptyInit
  (bind _tiles (Variables|Default|GetTiles))
  (if (Utilities|Array|IsEmpty _tiles)
    (for _index (range 0 15)
      (Utilities|Array|Add _tiles (Utilities|Struct|MakeGridOneDimension "(tiletype_5_369C74E94551080623A369B049E6C79E=NewEnumerator0)")))))

(fn GridtoWorld
  (params (Grid :type Vector))
  (return (* Grid "100.000000,100.000000,100.000000")))