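; BP_ATile is a grid tile actor, apparently a parent class, whose mesh depends on its tile type and season.
; ChangeOnType uses nested selects on Season and TileType to set the Cube's static mesh, with low season variants sharing their season's meshes.
; The construction script caches the BP_AGrid reference and refreshes the mesh.
; Init repeats both steps and records the starting season in OriginalSeason.
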(event EventBeginPlay)

(event Collision|EventActorBeginOverlap
  (params (OtherActor :type Actor%20Object%20Reference)))

(event EventTick
  (params (DeltaSeconds :type Float%20%28single-precision%29)))

(fn ConstructionScript
  (CallFunction|GetGrid)
  (CallFunction|ChangeonType))

(fn ChangeonType
  (bind _tiletype (Variables|Default|GetTileType))
  (bind _returnvalue (Utilities|Select :Index _tiletype :NewEnumerator0 "/Game/Art/Environment/playGround/Mesh/SM_Ground_Summer.SM_Ground_Summer" :NewEnumerator1 "/Game/Art/Environment/playGround/Mesh/SM_Hole_Summer.SM_Hole_Summer" :NewEnumerator2 "/Game/Art/Environment/Summer/Meshes/Towel.Towel" :NewEnumerator3 "/Game/Art/Environment/playGround/Mesh/SM_Path_Summer.SM_Path_Summer"))
  (bind _returnvalue_2 (Utilities|Select :Index _tiletype :NewEnumerator0 "/Game/Art/Environment/playGround/Mesh/SM_Ground_Winter.SM_Ground_Winter" :NewEnumerator1 "/Game/Art/Environment/playGround/Mesh/SM_Hole_Winter.SM_Hole_Winter" :NewEnumerator2 "/Game/Art/Environment/playGround/Mesh/SM_Ice_Block.SM_Ice_Block" :NewEnumerator3 "/Game/Art/Environment/playGround/Mesh/SM_Path_Winter.SM_Path_Winter"))
  (Components|StaticMesh|SetStaticMesh (Variables|Default|GetCube) (Utilities|Select :Index (Variables|Default|GetSeason) :NewEnumerator0 _returnvalue_2 :NewEnumerator1 _returnvalue_2 :NewEnumerator2 _returnvalue :NewEnumerator3 _returnvalue)))

(fn GetGrid
  (bind _returnvalue (Actor|GetActorOfClass "/Game/Core/Blueprints/Actor/Parent/BP_AGrid.BP_AGrid_C"))
  (Variables|Default|SetGridRef _returnvalue))

(fn Init
  (CallFunction|GetGrid)
  (CallFunction|ChangeonType)
  (Variables|Default|SetoriginalSeason (Variables|Default|GetSeason)))