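; BP_AProp is a parent actor for grid-based props that snap into place and test adjacency to the player.
; On BeginPlay it caches the BP_AGrid and player pawn, then teleports to its XY position snapped to 100-unit cells plus an offset, flattening Z to that offset.
; ClosedToPlayer compares prop and player cell coordinates, returning whether they are one cell apart and the player-to-prop direction, with debug prints of both.
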(event EventBeginPlay
  (bind _returnvalue (Actor|GetActorOfClass "/Game/Core/Blueprints/Actor/Parent/BP_AGrid.BP_AGrid_C"))
  (Variables|Default|SetGrid _returnvalue)
  (Variables|Default|SetPlayerPawn (Game|Player|GetPlayerPawn 0))
  (CallFunction|SetGridPos (Variables|Default|GetOffSet)))

(fn ConstructionScript)

(fn SetGridPos
  (params (Offset :type Vector))
  (bind _returnvalue (Transformation|GetActorLocation))
  (bind _returnvalue_2 (Class|KismetMathLibrary|VectorSnappedtoGrid _returnvalue 1e+02))
  (bind _returnvalue_3 (Transformation|SetActorLocation (+ Offset (Math|Vector|MakeVector (.x _returnvalue_2) (.y _returnvalue_2) 0.0)) false true))
  (return _returnvalue_3))

(fn ClosedtoPlayer
  (bind _gridpos (Utilities|GetActorPosGrid))
  (bind _posgrid (Utilities|GetPlayerPosGrid))
  (bind _returnvalue (- _gridpos _posgrid))
  (Development|PrintString (Utilities|String|ToString(Vector) _gridpos) true true "(R=1.000000,G=0.103669,B=0.000000,A=1.000000)" 0.0)
  (Development|PrintString (Utilities|String|ToString(Vector) _posgrid) true true "(R=0.000000,G=0.660000,B=1.000000,A=1.000000)" 0.0)
  (return (== (Math|Vector|VectorLength _returnvalue) 1.0) _returnvalue))