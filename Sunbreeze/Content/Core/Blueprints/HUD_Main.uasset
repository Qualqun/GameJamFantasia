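; Main HUD Blueprint that puts the W_HudGame widget on screen and switches it between gameplay and pause-style menu pages.
; On BeginPlay, a CreateWidget helper builds the widget for the first player, adds it to the viewport and stores it as HudUi.
; PauseMode sets the active HudSwitcher page, with any non-zero index showing the cursor and using UI-only input, and zero restoring game-only input.
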(event EventBeginPlay
  (bind _returnvalue (CallFunction|CreateWidget "/Game/Core/Blueprints/UI/W_HudGame.W_HudGame_C"))
  (bind _asw_hud_game (Utilities|Casting|CastToW_HudGame _returnvalue))
  (Variables|Default|SetHudUi _asw_hud_game))

(fn ConstructionScript)

(fn PauseMode
  (params (ActiveId :type Integer))
  (bind _returnvalue (Game|GetPlayerController 0))
  (bind _hudui (Variables|Default|GetHudUi))
  (bind _hudswitcher (Variables|/Game/Core/Blueprints/UI/W_HudGame.W_HudGame_C|GetHudSwitcher _hudui))
  (bind _output_get (Variables|/Script/UMG.WidgetSwitcher|SetActiveWidgetIndex _hudswitcher ActiveId))
  (bind _output_get_2 (Variables|/Script/Engine.PlayerController|SetbShowMouseCursor _returnvalue (Math|Conversions|ToBoolean(Integer) _output_get)))
  (if _output_get_2
    (Input|SetInputModeUIOnly _returnvalue _hudswitcher "DoNotLock" false)
    (else
      (Input|SetInputModeGameOnly _returnvalue false)))
  (return))

(fn CreateWidget
  (params (HUDWidget :type User%20Widget%20Class%20Reference))
  (bind _returnvalue (UserInterface|CreateWidget HUDWidget (Game|GetPlayerController 0)))
  (UserInterface|Viewport|AddtoViewport _returnvalue 0)
  (return _returnvalue))